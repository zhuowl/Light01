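; Sliding door Blueprint that opens when BP_PlayPawn enters DoorTrigger and closes when it leaves, gated by the Can flag.
; The Move timeline drives the Door mesh along a spline and calls UpdateLight on the level's Manger actor every update.
; A StopDoor volume halts the timeline when a tagged Prop_BP component overlaps it and reverses it once the prop leaves.
; PlaySound is an empty stub.
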(event OnComponentBeginOverlap(DoorTrigger)
  (params (OverlappedComponent :type Primitive%20Component%20Object%20Reference) (OtherActor :type Actor%20Object%20Reference) (OtherComp :type Primitive%20Component%20Object%20Reference) (OtherBodyIndex :type Integer) (bFromSweep :type Boolean) (SweepResult :type Hit%20Result%20Structure%20%28by%20ref%29))
  (if (Variables|Default|GetCan)
    (Utilities|Casting|CastToBP_PlayPawn OtherActor)
    (CallFunction|OpenDoor)
    (CallFunction|PlaySound)))

(event OnComponentEndOverlap(DoorTrigger)
  (params (OverlappedComponent :type Primitive%20Component%20Object%20Reference) (OtherActor :type Actor%20Object%20Reference) (OtherComp :type Primitive%20Component%20Object%20Reference) (OtherBodyIndex :type Integer))
  (if (Variables|Default|GetCan)
    (Utilities|Casting|CastToBP_PlayPawn OtherActor)
    (CallFunction|CloseDoor)))

(event OnComponentBeginOverlap(StopDoor)
  (params (OverlappedComponent :type Primitive%20Component%20Object%20Reference) (OtherActor :type Actor%20Object%20Reference) (OtherComp :type Primitive%20Component%20Object%20Reference) (OtherBodyIndex :type Integer) (bFromSweep :type Boolean) (SweepResult :type Hit%20Result%20Structure%20%28by%20ref%29))
  (Utilities|Casting|CastToProp_BP OtherActor)
  (if (Components|ComponentHasTag (Transformation|GetAttachParent OtherComp) "Prop")
    (CallFunction|Stop)))

(event OnComponentEndOverlap(StopDoor)
  (params (OverlappedComponent :type Primitive%20Component%20Object%20Reference) (OtherActor :type Actor%20Object%20Reference) (OtherComp :type Primitive%20Component%20Object%20Reference) (OtherBodyIndex :type Integer))
  (Utilities|Casting|CastToProp_BP OtherActor)
  (if (Components|ComponentHasTag (Transformation|GetAttachParent OtherComp) "Prop")
    (Utilities|String|Reverse (Variables|Default|GetMove))))

(event Custom|OpenDoor
  (bind _spline (Variables|Default|GetSpline))
  ;[1 1 1] 门的开合
  (bind _newtrack_0 (Timeline|Move Play)
    (:Update
      (Default|UpdateLight (Variables|Default|GetManger))
      (Transformation|SetWorldLocation (Variables|Default|GetDoor) (Spline|GetLocationatDistanceAlongSpline _spline (Math|Float|Lerp 0.0 (Spline|GetSplineLength _spline) _newtrack_0) "World") false false))))

(event Custom|PlaySound)

(event Custom|CloseDoor
  (bind _spline (Variables|Default|GetSpline))
  ;[1 1 1] 门的开合
  (bind _newtrack_0 (Timeline|Move ReverseFromEnd)
    (:Update
      (Default|UpdateLight (Variables|Default|GetManger))
      (Transformation|SetWorldLocation (Variables|Default|GetDoor) (Spline|GetLocationatDistanceAlongSpline _spline (Math|Float|Lerp 0.0 (Spline|GetSplineLength _spline) _newtrack_0) "World") false false))))

(event Custom|stop
  (bind _spline (Variables|Default|GetSpline))
  ;[1 1 1] 门的开合
  (bind _newtrack_0 (Timeline|Move Stop)
    (:Update
      (Default|UpdateLight (Variables|Default|GetManger))
      (Transformation|SetWorldLocation (Variables|Default|GetDoor) (Spline|GetLocationatDistanceAlongSpline _spline (Math|Float|Lerp 0.0 (Spline|GetSplineLength _spline) _newtrack_0) "World") false false))))

(event EventBeginPlay
  (bind _outactors (Actor|GetAllActorsOfClass "/Game/Manger.Manger_C"))
  (Variables|Default|SetManger (Utilities|Array|Get(acopy) _outactors)))

(event Collision|EventActorBeginOverlap
  (params (OtherActor :type Actor%20Object%20Reference)))

(event EventTick
  (params (DeltaSeconds :type Float%20%28single-precision%29)))

(fn ConstructionScript)