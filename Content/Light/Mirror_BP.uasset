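; Clickable mirror for a light puzzle that the player can rotate to redirect light.
; Overlap of the player's DoingTrigger with InfereneTrigger swaps the mesh to a Reflect material, restored on exit, and shows the Manger's mirror UI once.
; A Rotate+ event turns the mirror in fixed, swept steps while those triggers overlap.
; Clicking the mirror or mesh calls Rotate, then has the Manger update the light.
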(event OnComponentEndOverlap(InfereneTrigger)
  (params (OverlappedComponent :type Primitive%20Component%20Object%20Reference) (OtherActor :type Actor%20Object%20Reference) (OtherComp :type Primitive%20Component%20Object%20Reference) (OtherBodyIndex :type Integer))
  (if (== OtherActor (Variables|Default|GetPlayer))
    (Rendering|Material|SetMaterial (Variables|Default|GetStaticMesh) 0 (Variables|Default|GetTempMaterial))))

(event OnClicked(StaticMesh)
  (params (TouchedComponent :type Primitive%20Component%20Object%20Reference) (ButtonPressed :type Key%20Structure :default "AnyKey"))
  (CallFunction|Rotate+)
  (Default|UpdateLight (Variables|Default|GetManger)))

(event OnClicked(Mirror)
  (params (TouchedComponent :type Primitive%20Component%20Object%20Reference) (ButtonPressed :type Key%20Structure :default "AnyKey"))
  (CallFunction|Rotate+)
  (Default|UpdateLight (Variables|Default|GetManger)))

(event OnComponentBeginOverlap(InfereneTrigger)
  (params (OverlappedComponent :type Primitive%20Component%20Object%20Reference) (OtherActor :type Actor%20Object%20Reference) (OtherComp :type Primitive%20Component%20Object%20Reference) (OtherBodyIndex :type Integer) (bFromSweep :type Boolean) (SweepResult :type Hit%20Result%20Structure%20%28by%20ref%29))
  (if (== OtherComp (Variables|Default|GetDoingTrigger))
    (Rendering|Material|SetMaterial (Variables|Default|GetStaticMesh) 0 "/Game/Geometry/Meshes/Reflect.Reflect")
    (Utilities|FlowControl|DoOnce false
      (:Completed
        (Default|MirrorUI (Variables|Default|GetManger))))))

(event Custom|Rotate+
  ;[1 1 1] 旋转事件
  (if (Class|PrimitiveComponent|IsOverlappingComponent (Variables|Default|GetInfereneTrigger) (Variables|Default|GetDoingTrigger))
    (Transformation|AddRelativeRotation (Variables|Default|GetMirror) "0,5.000000, 0" true false)))

(event EventBeginPlay
  (Utilities|FlowControl|Sequence
    (:then_0
      (Variables|Default|SetTempMaterial (Rendering|Material|GetMaterial (Variables|Default|GetStaticMesh) (Variables|Default|GetMaterialIndex))))
    (:then_1
      ;[1 1 1] 获取玩家
      (bind _asbp_play_pawn (Utilities|Casting|CastToBP_PlayPawn (Game|Player|GetPlayerPawn 0)))
      (bind _output_get (Variables|Default|SetPlayer _asbp_play_pawn))
      (Variables|Default|SetDoingTrigger (Variables|/Game/player/Blueprints/BP_PlayPawn.BP_PlayPawn_C|GetDoingTrigger _output_get)))
    (:then_2
      (bind _outactors (Actor|GetAllActorsOfClass "/Game/Manger.Manger_C"))
      (Variables|Default|SetManger (Utilities|Array|Get(acopy) _outactors)))))

(event Collision|EventActorBeginOverlap
  (params (OtherActor :type Actor%20Object%20Reference)))

(fn ConstructionScript
  (|CallParentFunction))