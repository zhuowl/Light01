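; BP_Player is the player character, which carries props, chisels walls and rotates mirrors.
; Construction attaches the awl and GetScene to mesh sockets, and BeginPlay caches the Manger actor.
; Prop and wall actions act on the first actor whose state flag allows it, with walk speed changing while carrying.
; Movement follows control yaw and cancels chiseling, turning clamps camera pitch, and mirrors are found by trigger overlap.
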(event EventBeginPlay
  (bind _outactors (Actor|GetAllActorsOfClass "/Game/Manger.Manger_C"))
  (Variables|Default|SetManger (Utilities|Array|Get(acopy) _outactors)))

(event Collision|EventActorBeginOverlap
  (params (OtherActor :type Actor%20Object%20Reference)))

(fn ConstructionScript
  (Utilities|FlowControl|Sequence
    (:then_0
      (Transformation|AttachComponentToComponent (Variables|Default|Getawl) (Variables|Character|GetMesh) "Chisel" "KeepRelative" "KeepRelative" "KeepRelative" true))
    (:then_1
      (Transformation|AttachComponentToComponent (Variables|Default|GetGetScene) (Variables|Character|GetMesh) "Prop" "KeepRelative" "KeepWorld" "KeepWorld" true))
    (:then_2
      (Variables|/Script/Engine.CharacterMovementComponent|SetMaxWalkSpeed (Variables|Character|GetCharacterMovement) (Variables|Default|GetmaxSpeed_Normal)))))

(fn GetProp
  (bind _outactors (Actor|GetAllActorsOfClass "/Game/BP_Prop.BP_Prop_C"))
  (bind _array_element (Utilities|Array|ForEachLoopwithBreak _outactors :!label _label)
    (:LoopBody
      (if (Variables|/Game/BP_Prop.BP_Prop_C|GetCan _array_element)
        (Default|BeGot _array_element)
        (Utilities|FlowControl|Sequence
          (:then_0
            (Variables|/Script/Engine.CharacterMovementComponent|SetMaxWalkSpeed (Variables|Character|GetCharacterMovement) (Variables|Default|GetmaxSpeed_Prop)))
          (:then_1
            (Variables|Default|SetIsGeting true)
            (goto _label Break)))))))

(fn PutProp
  ;[1 1 1] 放下道具
  (bind _outactors (Actor|GetAllActorsOfClass "/Game/BP_Prop.BP_Prop_C"))
  (bind _array_element (Utilities|Array|ForEachLoopwithBreak _outactors :!label _label)
    (:LoopBody
      (if (Variables|/Game/BP_Prop.BP_Prop_C|Getbeing _array_element)
        (Default|BeDrop _array_element)
        (Utilities|FlowControl|Sequence
          (:then_0
            (Variables|/Script/Engine.CharacterMovementComponent|SetMaxWalkSpeed (Variables|Character|GetCharacterMovement) (Variables|Default|GetmaxSpeed_Normal)))
          (:then_1
            (Variables|Default|SetIsGeting false)
            (goto _label Break)))))))

(fn Chisel
  ;[1 1 1] Chisel/凿墙
  (bind _outactors (Actor|GetAllActorsOfClass "/Game/wall/BluePrints/Wall.Wall_C"))
  (bind _array_element (Utilities|Array|ForEachLoopwithBreak _outactors :!label _label)
    (:LoopBody
      (if (Variables|/Game/wall/BluePrints/Wall.Wall_C|GetCan _array_element)
        (Variables|/Game/wall/BluePrints/Wall.Wall_C|SetisChisel _array_element true)
        (Variables|Default|SetisChiesl true)
        (goto _label Break)))))

(fn Move
  (params (forward :type Float%20%28single-precision%29) (Right :type Float%20%28single-precision%29))
  (bind _returnvalue (Pawn|GetControlRotation :!class /Script/Engine.Pawn))
  (bind _yaw (Math|Rotator|BreakRotator _returnvalue))
  (bind _returnvalue_2 (Math|Rotator|MakeRotator 0.0 0.0 _yaw))
  ;[1 1 1] Movement input/移动输入
  (Variables|Default|Setforward forward)
  (Variables|Default|Setright Right)
  (Utilities|FlowControl|Sequence
    (:then_0
      (Pawn|Input|AddMovementInput (Math|Vector|GetForwardVector _returnvalue_2) (Variables|Default|Getforward) false))
    (:then_1
      (Pawn|Input|AddMovementInput (Math|Vector|GetRightVector _returnvalue_2) (Variables|Default|Getright) false)))
  (if (or (!= (Variables|Default|Getforward) 0.0) (!= (Variables|Default|Getright) 0.0))
    (Variables|Default|SetisChiesl false)))

(fn RotateMirror
  (params (Z :type Float%20%28single-precision%29))
  (bind _asbp_mirror (Utilities|Casting|CastToBP_Mirror (Utilities|Array|Get(acopy) (Collision|GetOverlappingActors (Variables|Default|GetGettingTrigger) "/Game/BP_Mirror.BP_Mirror_C" :!class /Script/Engine.PrimitiveComponent))))
  (Default|Turn _asbp_mirror Z))

(fn Turn
  (params (Yaw :type Float%20%28single-precision%29) (Pitch :type Float%20%28single-precision%29))
  (bind _returnvalue (Game|GetPlayerController 0))
  (bind _returnvalue_2 (Pawn|GetControlRotation _returnvalue :!class /Script/Engine.Controller))
  ;[1 1 1] Turn/转向控制
  (Utilities|FlowControl|Sequence
    (:then_0
      (Pawn|Input|AddControllerYawInput (* Yaw (Variables|Default|GetBaseTurnRate) (Utilities|Time|GetWorldDeltaSeconds))))
    (:then_1
      (Pawn|Input|AddControllerPitchInput (* Pitch (Variables|Default|GetBaseLookUpRate) (Utilities|Time|GetWorldDeltaSeconds)))
      (Pawn|SetControlRotation _returnvalue (Math|Rotator|MakeRotator (.roll _returnvalue_2) (+ (Math|Float|ClampAngle (- (.pitch _returnvalue_2) 1.8e+02) 145.0 -1.6e+02) 1.8e+02) (.yaw _returnvalue_2))))))