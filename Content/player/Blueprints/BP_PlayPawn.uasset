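; Player pawn with click-to-move, prop carrying, camera rotation and a wall-chisel state.
; Clicks on Floor-tagged components set a target that Tick steers toward via physics velocity, while Wall-tagged hits set IsChisel.
; W picks up or drops an overlapping Prop, rescaling it on a body-socketed scene point and telling the Manger actor to update lighting.
; One-shot gates on mouse release, A/D release and wall overlap trigger Manger UI calls.
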(event OnComponentBeginOverlap(DoingTrigger)
  (params (OverlappedComponent :type Primitive%20Component%20Object%20Reference) (OtherActor :type Actor%20Object%20Reference) (OtherComp :type Primitive%20Component%20Object%20Reference) (OtherBodyIndex :type Integer) (bFromSweep :type Boolean) (SweepResult :type Hit%20Result%20Structure%20%28by%20ref%29))
  (Utilities|FlowControl|Sequence
    (:then_0
      (if (Components|ComponentHasTag OtherComp "Wall")
        (Utilities|FlowControl|DoOnce false
          (:Completed
            (Default|HoleUI (Variables|Default|GetManger))))))))

(event Custom|GetProp
  ;[1 1 1] 拿起道具
  (bind _array_element (Utilities|Array|ForEachLoopwithBreak (Class|PrimitiveComponent|GetOverlappingComponents (Variables|Default|GetDoingTrigger)) :!label _label)
    (:LoopBody
      (if (Components|ComponentHasTag _array_element "Prop")
        (bind _output_get (Variables|Default|SetProp (Transformation|GetAttachParent _array_element)))
        (Variables|Default|SetTempZ (.Z (Math|Vector|BreakVector (Transformation|GetWorldLocation (Transformation|GetAttachParent _array_element)))))
        (Transformation|SetWorldLocation _output_get (Transformation|GetWorldLocation (Variables|Default|GetGetScene)) false false)
        (Transformation|SetWorldScale3D (Variables|Default|GetProp) (/ (Transformation|GetWorldScale (Transformation|GetAttachParent _array_element)) (Variables|Default|GetTempSize)))
        (Transformation|AttachComponentToComponent (Variables|Default|GetProp) (Variables|Default|GetGetScene) "None" "KeepWorld" "KeepRelative" "KeepRelative" true)
        (Rendering|SetVisibility (Variables|Default|Gettarget) true false)
        (Variables|Default|SetIsGeting true)
        (goto _label Break)))
    (:Completed
      (Default|UpdateLight (Variables|Default|GetManger)))))

(event Custom|CantMove
  (Variables|Default|SetSpeed 0.0))

(event Custom|PutProp
  (bind _putscene (Variables|Default|GetPutScene))
  (bind _prop (Variables|Default|GetProp))
  (bind _returnvalue (Transformation|GetWorldLocation _putscene))
  (bind (_x _y) (Math|Vector|BreakVector _returnvalue))
  ;[1 1 1] 放下道具
  (Class|SceneComponent|DetachfromParent _prop false true)
  (Transformation|SetWorldLocation _prop (Math|Vector|MakeVector _x _y (Variables|Default|GetTempZ)) false false)
  (Transformation|SetWorldRotation (Variables|Default|GetProp) (Transformation|GetWorldRotation (Variables|Default|GetPutScene)) false false)
  (Transformation|SetWorldScale3D (Variables|Default|GetProp) (* (Transformation|GetWorldScale (Variables|Default|GetProp)) (Variables|Default|GetTempSize)))
  (Variables|Default|SetIsGeting false)
  (Default|UpdateLight (Variables|Default|GetManger))
  (Rendering|SetVisibility (Variables|Default|Gettarget) false false))

(event Collision|EventActorBeginOverlap
  (params (OtherActor :type Actor%20Object%20Reference)))

(event EventTick
  (params (DeltaSeconds :type Float%20%28single-precision%29))
  (bind _targetposition (Variables|Default|GetTargetPosition))
  (bind _capsulecollision (Variables|Default|GetCapsuleCollision))
  (bind _returnvalue (Transformation|GetWorldLocation _capsulecollision))
  (bind _returnvalue_2 (- _targetposition _returnvalue))
  (bind _returnvalue_3 (Math|Vector|Normalize _returnvalue_2))
  (bind (_x _y) (Math|Vector|BreakVector _returnvalue_2))
  (bind (_x_2 _y_2) (Math|Vector|BreakVector _returnvalue_3))
  ;[1 1 1] 获得按键的值给相应的 移动方向加上velocity
  (if (> (Math|Vector|VectorLength (Math|Vector|MakeVector _x _y 0.0)) 0.0)
    (Physics|SetPhysicsLinearVelocity (Variables|Default|GetCapsuleCollision) (* (Math|Vector|MakeVector _x_2 _y_2 0.0) (Variables|Default|GetSpeed)) false "None")
    ;[1 1 1] 改变角色的朝向
    (Transformation|SetWorldRotation (Variables|Default|GetCapsuleCollision) (Math|Rotator|MakeRotator 0.0 0.0 (.Yaw (Math|Rotator|BreakRotator (Math|Rotator|FindLookatRotation (Transformation|GetWorldLocation (Variables|Default|GetCapsuleCollision)) (Variables|Default|GetTargetPosition))))) false false)
    (else
      (Physics|SetPhysicsLinearVelocity (Variables|Default|GetCapsuleCollision) "0, 0, 0" false "None"))))

(event EventBeginPlay
  ;[1 1 1] 游戏的初始设置
  (Variables|Default|SetTargetPosition (Transformation|GetWorldLocation (Variables|Default|GetCapsuleCollision)))
  (bind _outactors (Actor|GetAllActorsOfClass "/Game/Manger.Manger_C"))
  (Variables|Default|SetManger (Utilities|Array|Get(acopy) _outactors)))

(event Input|AxisEvents|InputAxisTurnLeft
  (params (AxisValue :type Float%20%28single-precision%29))
  ;[1 1 1] 旋转视野
  (Transformation|AddWorldRotation (Variables|Default|GetSpringArm) (Math|Rotator|MakeRotator 0.0 0.0 AxisValue) false false))

(event Input|KeyboardEvents|W
  (params (Key :type Key%20Structure :default "AnyKey"))
  (:Pressed
    (if (Variables|Default|GetIsGeting)
      (CallFunction|PutProp)
      (else
        (CallFunction|GetProp)))))

(event Input|KeyboardEvents|A
  (params (Key :type Key%20Structure :default "AnyKey"))
  (:Released
    (Utilities|FlowControl|DoOnce false
      (:Completed
        (Utilities|FlowControl|Delay 1.0)
        (Default|WinTurmUI (Variables|Default|GetManger))))))

(event Input|MouseEvents|LeftMouseButton
  (params (Key :type Key%20Structure :default "AnyKey"))
  (bind _returnvalue (Game|GetPlayerController 0))
  (bind _hitresult (Game|Player|GetHitResultUnderCursorbyChannel _returnvalue "TraceTypeQuery1" true))
  (bind (_bblockinghit _binitialoverlap _time _location _impactpoint _normal _impactnormal _physmat _hitactor _hitcomponent) (Collision|BreakHitResult _hitresult))
  (:Pressed
    ;[1 1 1] 鼠标点下的点 为目标点// 凿墙 和 移动
    (if _bblockinghit
      (switch name (Utilities|Array|Get(acopy) (Variables|/Script/Engine.ActorComponent|GetComponentTags _hitcomponent))
        (:Floor
          (bind _output_get (Variables|Default|SetTargetPosition _location))
          (Effects|SpawnEmitteratLocation "/Game/StarterContent/Particles/P_Mouse.P_Mouse" _output_get "0, 0,0.000000")
          (Variables|Default|SetIsChisel false))
        (:Wall
          (Variables|Default|SetIsChisel true)))))
  (:Released
    (Utilities|FlowControl|Delay 0.2)
    (Variables|Default|SetIsChisel false)
    (Utilities|FlowControl|DoOnce false
      (:Completed
        (Default|TurnViewUI (Variables|Default|GetManger))))))

(event Input|KeyboardEvents|D
  (params (Key :type Key%20Structure :default "AnyKey"))
  (:Released
    (Utilities|FlowControl|DoOnce false
      (:Completed
        (Utilities|FlowControl|Delay 1.0)
        (Default|WinTurmUI (Variables|Default|GetManger))))))

(fn ConstructionScript
  (bind _playerbody (Variables|Default|GetPlayerBody))
  (Transformation|AttachComponentToComponent (Variables|Default|Getawl) _playerbody "Chisel" "KeepRelative" "KeepRelative" "KeepRelative" true)
  (Transformation|AttachComponentToComponent (Variables|Default|GetGetScene) _playerbody "Prop" "KeepRelative" "KeepWorld" "KeepWorld" true))