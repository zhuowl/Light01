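; Rotatable mirror actor for a light puzzle, which updates the light through a Manger actor found at BeginPlay.
; Overlap with DoingTrigger swaps the mesh to a Reflect material and triggers the mirror UI once; the player leaving restores the saved material.
; Clicking either mesh calls Rotate and UpdateLight.
; Separate events turn the mirror by frame-time-scaled yaw or a fixed step gated on overlap.
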(event OnComponentEndOverlap(InfereneTrigger)
  (params (OverlappedComponent :type Primitive%20Component%20Object%20Reference) (OtherActor :type Actor%20Object%20Reference) (OtherComp :type Primitive%20Component%20Object%20Reference) (OtherBodyIndex :type Integer))
  (if (== OtherActor (Variables|Default|GetPlayer))
    (Rendering|Material|SetMaterial (Variables|Default|GetStaticMesh) 0 (Variables|Default|GetTempMaterial))))

(event OnClicked(StaticMesh)
  (params (TouchedComponent :type Primitive%20Component%20Object%20Reference) (ButtonPressed :type Key%20Structure :default "AnyKey"))
  (CallFunction|Rotate+)
  (Default|UpdateLight (Variables|Default|GetManger)))

(event OnClicked(Mirror)
  (params (TouchedComponent :type Primitive%20Component%20Object%20Reference) (ButtonPressed :type Key%20Structure :default "AnyKey"))
  (CallFunction|Rotate+)
  (Default|UpdateLight (Variables|Default|GetManger)))

(event OnComponentBeginOverlap(InfereneTrigger)
  (params (OverlappedComponent :type Primitive%20Component%20Object%20Reference) (OtherActor :type Actor%20Object%20Reference) (OtherComp :type Primitive%20Component%20Object%20Reference) (OtherBodyIndex :type Integer) (bFromSweep :type Boolean) (SweepResult :type Hit%20Result%20Structure%20%28by%20ref%29))
  (if (== OtherComp (Variables|Default|GetDoingTrigger))
    (Rendering|Material|SetMaterial (Variables|Default|GetStaticMesh) 0 "/Game/Geometry/Meshes/Reflect.Reflect")
    (Utilities|FlowControl|DoOnce false
      (:Completed
        (Default|MirrorUI (Variables|Default|GetManger))))))

(event Custom|Rotate+
  ;[1 1 1] 旋转事件
  (if (Class|PrimitiveComponent|IsOverlappingComponent (Variables|Default|GetInfereneTrigger) (Variables|Default|GetDoingTrigger))
    (Transformation|AddRelativeRotation (Variables|Default|GetMirror) "0,5.000000, 0" true false)))

(event Custom|turn
  (params (NewParam :type Float%20%28single-precision%29))
  (Transformation|AddWorldRotation (Variables|Default|GetMirror) (Math|Rotator|MakeRotator 0.0 0.0 (* NewParam (Utilities|Time|GetWorldDeltaSeconds) (Variables|Default|GetNewVar_2))) false false))

(event EventBeginPlay
  (Utilities|FlowControl|Sequence
    (:then_0
      (Variables|Default|SetTempMaterial (Rendering|Material|GetMaterial (Variables|Default|GetStaticMesh) (Variables|Default|GetMaterialIndex))))
    (:then_2
      (bind _outactors (Actor|GetAllActorsOfClass "/Game/Manger.Manger_C"))
      (Variables|Default|SetManger (Utilities|Array|Get(acopy) _outactors)))))

(event Collision|EventActorBeginOverlap
  (params (OtherActor :type Actor%20Object%20Reference)))

(event EventTick
  (params (DeltaSeconds :type Float%20%28single-precision%29)))

(fn ConstructionScript
  (|CallParentFunction))