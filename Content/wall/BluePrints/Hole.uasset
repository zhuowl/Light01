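; Hole is a scene component for walls that checks which light sources have a clear line to its position.
; On BeginPlay, FoundLight gathers actors tagged "illuminant" and runs a complex Visibility trace from the component to each, with debug lines drawn.
; A hit on a tagged actor leads only to an owner validity check with no action after it, so detection has no effect yet.
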(event EventBeginPlay
  (CallFunction|FoundLight))

(event EventTick
  (params (DeltaSeconds :type Float%20%28single-precision%29)))

(fn FoundLight
  ;[1 1 1] Found Light
  (bind _outactors (Actor|GetAllActorswithTag "illuminant"))
  (bind _output_get (Variables|Default|Setilluminants _outactors))
  (for _array_element _output_get
    (bind _outhit (Collision|LineTraceByChannel (Transformation|GetWorldLocation) (Transformation|GetActorLocation _array_element) "TraceTypeQuery1" true 0 "ForDuration" true "(R=1.000000,G=0.000000,B=0.000000,A=1.000000)" "(R=0.000000,G=1.000000,B=0.000000,A=1.000000)" 1e+02))
    (if (and (.bBlockingHit (Collision|BreakHitResult _outhit)) (Actor|ActorHasTag (.HitActor (Collision|BreakHitResult _outhit)) "illuminant"))
      (Utilities|IsValid (Components|GetOwner)))))