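; Chiselable wall that the player breaks through, after which it can send out a laser of light.
; Tick accumulates time while the player's trigger overlaps the wall and IsChisel is set; once past Quality, ChiselFinished swaps in the holed mesh and clears the player's chisel flag.
; A separate Finished event swaps to NewWall and spawns a SpawnLight laser from ArrowOut, aimed horizontally away from the overlapping BP_illuminant.
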(event Custom|Finished
  (bind _arrowout (Variables|Default|GetArrowOut))
  (bind _returnvalue (Transformation|GetWorldLocation _arrowout))
  ;[1 1 1] 凿墙结束后发出光线
  (Components|StaticMesh|SetStaticMesh (Variables|Default|Getwall) (Variables|Default|GetNewWall))
  (bind _asbp_illuminant (Utilities|Casting|CastToBP_illuminant (Utilities|Array|Get(acopy) (Collision|GetOverlappingActors "/Game/Blueprint/BP_illuminant.BP_illuminant_C" :!class /Script/Engine.Actor))))
  (bind _returnvalue_2 (Game|SpawnActorfromClass "/Game/Light/SpawnLight.SpawnLight_C" (Math|Transform|MakeTransform _returnvalue "0, 0, 0" "1,1,1") "Undefined" 0 0))
  (Default|SpawnLaser _returnvalue_2 _returnvalue (+ _returnvalue (* (Math|Vector|MakeVector (.X (Math|Vector|BreakVector (Math|Vector|Normalize (- _returnvalue (Transformation|GetActorLocation _asbp_illuminant))))) (.Y (Math|Vector|BreakVector (Math|Vector|Normalize (- _returnvalue (Transformation|GetActorLocation _asbp_illuminant))))) 0.0) 5e+03))))

(event EventBeginPlay
  ;[1 1 1] 游戏开始
  (Utilities|FlowControl|Sequence
    (:then_0
      (bind _asbp_player (Utilities|Casting|CastToBP_Player (Game|Player|GetPlayerPawn 0)))
      (Variables|Default|SetplayerPawn _asbp_player))
    (:then_1
      (bind _outactors (Actor|GetAllActorsOfClass "/Game/Manger.Manger_C"))
      (Variables|Default|SetManger (Utilities|Array|Get(acopy) _outactors)))))

(event Collision|EventActorBeginOverlap
  (params (OtherActor :type Actor%20Object%20Reference)))

(event EventTick
  (params (DeltaSeconds :type Float%20%28single-precision%29))
  (Utilities|FlowControl|Sequence
    (:then_0
      (Variables|Default|SetCan (Class|PrimitiveComponent|IsOverlappingComponent (Variables|Default|GetTrigger) (Variables|/Game/player/Blueprints/BP_Player.BP_Player_C|GetGettingTrigger (Variables|Default|GetplayerPawn)))))
    (:then_1
      (if (and (Variables|Default|GetCan) (Variables|Default|GetisChisel))
        (Variables|Default|SetTimer (+ (Variables|Default|GetTimer) (Utilities|Time|GetWorldDeltaSeconds)))))
    (:then_2
      (if (> (Variables|Default|GetTimer) (Variables|Default|Getquality))
        (Variables|Default|SetCan false)
        (Utilities|FlowControl|DoOnce false
          (:Completed
            (CallFunction|ChiselFinished)))))))

(fn ConstructionScript)

(fn ChiselFinished
  (Components|StaticMesh|SetStaticMesh (Variables|Default|Getwall) (Variables|Default|GetwallWithHole))
  (Variables|/Game/player/Blueprints/BP_Player.BP_Player_C|SetisChiesl (Variables|Default|GetplayerPawn) false))