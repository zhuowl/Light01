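; BP_Prop is a prop that the player can pick up and put down.
; Each tick it sets Can from whether its Trigger overlaps the player's GettingTrigger.
; BeGot shrinks the mesh by SmallRate and attaches it to the player's "Prop" socket, flagging Being.
; BeDrop detaches it, places it at PutScene with a 90-degree yaw offset, restores the scale cached at construction and clears the flag.
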(event EventBeginPlay
  (Utilities|FlowControl|Sequence
    (:then_0
      (Variables|Default|SetTempMaterial (Rendering|Material|GetMaterial (Variables|Default|GetProp) (Variables|Default|GetMaterialIndex))))
    (:then_1
      (bind _asbp_player (Utilities|Casting|CastToBP_Player (Game|Player|GetPlayerPawn 0)))
      (Variables|Default|SetplayerPawn _asbp_player))))

(event Collision|EventActorBeginOverlap
  (params (OtherActor :type Actor%20Object%20Reference)))

(event EventTick
  (params (DeltaSeconds :type Float%20%28single-precision%29))
  (Variables|Default|SetCan (Class|PrimitiveComponent|IsOverlappingComponent (Variables|Default|GetTrigger) (Variables|/Game/player/Blueprints/BP_Player.BP_Player_C|GetGettingTrigger (Variables|Default|GetplayerPawn)))))

(fn ConstructionScript
  (bind _output_get (Variables|Default|SettureScale (Transformation|GetWorldScale (Variables|Default|GetProp))))
  (Variables|Default|SetsmallScale (/ _output_get (Variables|Default|GetsmallRate))))

(fn BeDrop
  (bind _prop (Variables|Default|GetProp))
  (bind _playerpawn (Variables|Default|GetplayerPawn))
  (bind _putscene (Variables|/Game/player/Blueprints/BP_Player.BP_Player_C|GetPutScene _playerpawn))
  (bind _returnvalue (Transformation|GetWorldRotation _putscene))
  ;[1 1 1] 道具被放下
  (Utilities|FlowControl|Sequence
    (:then_0
      (Class|SceneComponent|DetachfromParent _prop false true))
    (:then_1
      (Transformation|SetWorldLocation _prop (Transformation|GetWorldLocation _putscene) false false))
    (:then_2
      (Transformation|SetWorldRotation _prop (Math|Rotator|MakeRotator (.roll _returnvalue) (.pitch _returnvalue) (+ (.yaw _returnvalue) 9e+01)) false false))
    (:then_3
      (Transformation|SetWorldScale3D _prop (Variables|Default|GettureScale)))
    (:then_4
      (Variables|Default|Setbeing false))))

(fn BeGot
  (bind _playerpawn (Variables|Default|GetplayerPawn))
  ;[1 1 1] 道具被拿起
  (Utilities|FlowControl|Sequence
    (:then_0
      (Transformation|SetWorldScale3D (Variables|Default|GetProp) (Variables|Default|GetsmallScale)))
    (:then_1
      (Transformation|SetWorldLocation (Variables|Default|GetDefaultSceneRoot) (Transformation|GetWorldLocation (Variables|/Game/player/Blueprints/BP_Player.BP_Player_C|GetGetScene _playerpawn)) false false))
    (:then_2
      (Transformation|AttachComponentToComponent (Variables|Default|GetProp) (Variables|/Script/Engine.Character|GetMesh _playerpawn) "Prop" "SnapToTarget" "KeepRelative" "KeepWorld" true))
    (:then_3
      (Variables|Default|Setbeing true))))