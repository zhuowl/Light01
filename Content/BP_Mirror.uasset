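; BP_Mirror is a rotatable mirror Actor that appears to be part of a light-reflection mechanic.
; Its Turn function yaws the Prop component by the input, scaled by TurnRate and frame delta time, using a swept rotation, unless the Being flag is set.
; After each rotation it calls UpdateLight on its Manger reference so the light is updated.
; Event graph and construction script add no logic of their own.
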(event EventBeginPlay
  (|CallParentFunction))

(event Collision|EventActorBeginOverlap
  (params (OtherActor :type Actor%20Object%20Reference)))

(event EventTick
  (params (DeltaSeconds :type Float%20%28single-precision%29)))

(fn ConstructionScript
  (|CallParentFunction))

(fn Turn
  (params (Z :type Float%20%28single-precision%29))
  (if (not (Variables|Default|Getbeing))
    (Transformation|AddWorldRotation (Variables|Default|GetProp) (Math|Rotator|MakeRotator 0.0 0.0 (* Z (Utilities|Time|GetWorldDeltaSeconds) (Variables|Default|GetturnRate))) true false)
    (Default|UpdateLight (Variables|Default|GetManger))))