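; Prop actor that highlights itself while the player is near and notifies a manager.
; On BeginPlay it caches the prop's original material, the BP_PlayPawn player with its DoingTrigger, and the first manager actor found.
; DoingTrigger entering Trigger swaps in the Reflect material and, through DoOnce, calls the manager's GetUI only the first time.
; End overlap tests the whole player actor, not DoingTrigger, before restoring the original material.
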(event OnComponentEndOverlap(Trigger)
  (params (OverlappedComponent :type Primitive%20Component%20Object%20Reference) (OtherActor :type Actor%20Object%20Reference) (OtherComp :type Primitive%20Component%20Object%20Reference) (OtherBodyIndex :type Integer))
  (if (== OtherActor (Variables|Default|GetPlayer))
    (Rendering|Material|SetMaterial (Variables|Default|GetProp) (Variables|Default|GetMaterialIndex) (Variables|Default|GetTempMaterial))))

(event OnComponentBeginOverlap(Trigger)
  (params (OverlappedComponent :type Primitive%20Component%20Object%20Reference) (OtherActor :type Actor%20Object%20Reference) (OtherComp :type Primitive%20Component%20Object%20Reference) (OtherBodyIndex :type Integer) (bFromSweep :type Boolean) (SweepResult :type Hit%20Result%20Structure%20%28by%20ref%29))
  (if (== OtherComp (Variables|Default|GetDoingTrigger))
    (Rendering|Material|SetMaterial (Variables|Default|GetProp) (Variables|Default|GetMaterialIndex) "/Game/Geometry/Meshes/Reflect.Reflect")
    (Utilities|FlowControl|DoOnce false
      (:Completed
        (Default|GetUI (Variables|Default|GetManger))))))

(event EventBeginPlay
  (Utilities|FlowControl|Sequence
    (:then_0
      (Variables|Default|SetTempMaterial (Rendering|Material|GetMaterial (Variables|Default|GetProp) (Variables|Default|GetMaterialIndex))))
    (:then_1
      ;[1 1 1] 获取玩家
      (bind _asbp_play_pawn (Utilities|Casting|CastToBP_PlayPawn (Game|Player|GetPlayerPawn 0)))
      (bind _output_get (Variables|Default|SetPlayer _asbp_play_pawn))
      (Variables|Default|SetDoingTrigger (Variables|/Game/player/Blueprints/BP_PlayPawn.BP_PlayPawn_C|GetDoingTrigger _output_get)))
    (:then_2
      (bind _outactors (Actor|GetAllActorsOfClass "/Game/Manger.Manger_C"))
      (Variables|Default|SetManger (Utilities|Array|Get(acopy) _outactors)))))

(event Collision|EventActorBeginOverlap
  (params (OtherActor :type Actor%20Object%20Reference)))

(event EventTick
  (params (DeltaSeconds :type Float%20%28single-precision%29)))

(fn ConstructionScript)