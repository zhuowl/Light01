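; BP_Door is a door that opens when the player's GettingTrigger component enters its DoorTrigger and closes when it leaves.
; A DoorMove timeline slides the Door along a spline by lerping distance over the spline's length, with closing running the timeline in reverse from its end.
; Each timeline update also calls UpdateLight on the Manger actor found at BeginPlay.
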(event OnComponentBeginOverlap(DoorTrigger)
  (params (OverlappedComponent :type Primitive%20Component%20Object%20Reference) (OtherActor :type Actor%20Object%20Reference) (OtherComp :type Primitive%20Component%20Object%20Reference) (OtherBodyIndex :type Integer) (bFromSweep :type Boolean) (SweepResult :type Hit%20Result%20Structure%20%28by%20ref%29))
  (if (== OtherComp (Variables|/Game/player/Blueprints/BP_Player.BP_Player_C|GetGettingTrigger (Variables|Default|GetplayerPawn)))
    (CallFunction|OpenDoor)))

(event OnComponentEndOverlap(DoorTrigger)
  (params (OverlappedComponent :type Primitive%20Component%20Object%20Reference) (OtherActor :type Actor%20Object%20Reference) (OtherComp :type Primitive%20Component%20Object%20Reference) (OtherBodyIndex :type Integer))
  (if (== OtherComp (Variables|/Game/player/Blueprints/BP_Player.BP_Player_C|GetGettingTrigger (Variables|Default|GetplayerPawn)))
    (CallFunction|CloseDoor)))

(event Custom|OpenDoor
  (bind _spline (Variables|Default|GetSpline))
  ;[1 1 1] 门的开合
  (bind _newtrack_0 (Timeline|doorMove Play)
    (:Update
      (Default|UpdateLight (Variables|Default|GetManger))
      (Transformation|SetWorldLocation (Variables|Default|GetDoor) (Spline|GetLocationatDistanceAlongSpline _spline (Math|Float|Lerp 0.0 (Spline|GetSplineLength _spline) _newtrack_0) "World") false false))))

(event Custom|CloseDoor
  (bind _spline (Variables|Default|GetSpline))
  ;[1 1 1] 门的开合
  (bind _newtrack_0 (Timeline|doorMove ReverseFromEnd)
    (:Update
      (Default|UpdateLight (Variables|Default|GetManger))
      (Transformation|SetWorldLocation (Variables|Default|GetDoor) (Spline|GetLocationatDistanceAlongSpline _spline (Math|Float|Lerp 0.0 (Spline|GetSplineLength _spline) _newtrack_0) "World") false false))))

(event Custom|stop
  (bind _spline (Variables|Default|GetSpline))
  ;[1 1 1] 门的开合
  (bind _newtrack_0 (Timeline|doorMove Stop)
    (:Update
      (Default|UpdateLight (Variables|Default|GetManger))
      (Transformation|SetWorldLocation (Variables|Default|GetDoor) (Spline|GetLocationatDistanceAlongSpline _spline (Math|Float|Lerp 0.0 (Spline|GetSplineLength _spline) _newtrack_0) "World") false false))))

(event EventBeginPlay
  ;[1 1 1] begin
  (Utilities|FlowControl|Sequence
    (:then_0
      (bind _outactors (Actor|GetAllActorsOfClass "/Game/Manger.Manger_C"))
      (Variables|Default|SetManger (Utilities|Array|Get(acopy) _outactors)))
    (:then_1
      (bind _asbp_player (Utilities|Casting|CastToBP_Player (Game|Player|GetPlayerPawn 0)))
      (Variables|Default|SetPlayerPawn _asbp_player))))

(event Collision|EventActorBeginOverlap
  (params (OtherActor :type Actor%20Object%20Reference)))

(event EventTick
  (params (DeltaSeconds :type Float%20%28single-precision%29)))

(fn ConstructionScript)