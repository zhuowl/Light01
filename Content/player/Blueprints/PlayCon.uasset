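; PlayCon is a player controller Blueprint that routes input to the possessed BP_Player pawn, which it casts and caches on BeginPlay.
; Axis inputs drive the pawn's movement, turning and mirror rotation, while the pickup action toggles between getting and putting down a prop.
; The wall/door action scans the pawn's trigger overlaps for a "door" tag but does nothing with it, leaving the Chisel call disconnected.
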(event EventBeginPlay
  ;[1 1 1] 获取被控制的PLayerPawn
  (bind _asbp_player (Utilities|Casting|CastToBP_Player (Pawn|GetControlledPawn)))
  (Variables|Default|SetPlayerPawn _asbp_player))

(event EventTick
  (params (DeltaSeconds :type Float%20%28single-precision%29)))

(event Input|ActionEvents|InputActionGetProps/drop
  (params (Key :type Key%20Structure :default "AnyKey"))
  (bind _playerpawn (Variables|Default|GetPlayerPawn))
  ;[1 1 1] 输入拾取/放下道具
  (:Pressed
    (if (Variables|/Game/player/Blueprints/BP_Player.BP_Player_C|GetIsGeting (Variables|Default|GetPlayerPawn))
      (Default|PutProp _playerpawn)
      (else
        (Default|GetProp _playerpawn)))))

(event Input|ActionEvents|InputActionwall/door
  (params (Key :type Key%20Structure :default "AnyKey"))
  ;[1 1 1] Chisel/凿墙
  (:Pressed
    (bind _array_element (Utilities|Array|ForEachLoopwithBreak (Class|PrimitiveComponent|GetOverlappingComponents (Variables|/Game/player/Blueprints/BP_Player.BP_Player_C|GetGettingTrigger (Variables|Default|GetPlayerPawn))) :!label _label)
      (:LoopBody
        (if (Components|ComponentHasTag _array_element "door")
          (goto _label Break))))))

(event Input|AxisEvents|InputAxisMoveForward
  (params (AxisValue :type Float%20%28single-precision%29))
  ;[1 1 1] Move/移动
  (Default|Move (Variables|Default|GetPlayerPawn) AxisValue (stale Input|AxisEvents|InputAxisMoveRight AxisValue)))

(event Input|AxisEvents|InputAxisRotateMirror
  (params (AxisValue :type Float%20%28single-precision%29))
  ;[1 1 1] 旋转镜子
  (Default|RotateMirror (Variables|Default|GetPlayerPawn) AxisValue))

(event Input|AxisEvents|InputAxisMoveRight
  (params (AxisValue :type Float%20%28single-precision%29))
  ;[1 1 1] Move/移动
  (Default|Move (Variables|Default|GetPlayerPawn) (stale Input|AxisEvents|InputAxisMoveForward AxisValue) AxisValue))

(event Input|AxisEvents|InputAxisTurnRate
  (params (AxisValue :type Float%20%28single-precision%29))
  (Default|Turn (Variables|Default|GetPlayerPawn) AxisValue (stale Input|AxisEvents|InputAxisLookUpRate AxisValue)))

(event Input|AxisEvents|InputAxisLookUpRate
  (params (AxisValue :type Float%20%28single-precision%29))
  (Default|Turn (Variables|Default|GetPlayerPawn) (stale Input|AxisEvents|InputAxisTurnRate AxisValue) AxisValue))

(fn ConstructionScript)